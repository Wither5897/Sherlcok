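; BP_Board is a board actor that opens the player's Reportboard UI when the player character walks into it.
; On BeginPlay it caches the player as TP_ThirdPersonCharacter; any actor overlap makes its own Widget1 visible.
; If the player overlaps while Reportboard is hidden, it shows that widget, switches to UI-only input with a mouse cursor and disables movement.
; It has no logic to close the board or restore control.
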(event EventBeginPlay
  (bind _astp_third_person_character (Utilities|Casting|CastToTP_ThirdPersonCharacter (Game|GetPlayerCharacter 0))))

(event EventTick
  (params (DeltaSeconds :type Float%20%28single-precision%29)))

(event Collision|EventActorBeginOverlap
  (params (OtherActor :type Actor%20Object%20Reference))
  (bind _returnvalue (Game|GetPlayerController 0))
  (Rendering|SetVisibility (Variables|Default|GetWidget1) true false)
  (if (and (== OtherActor (stale EventBeginPlay _astp_third_person_character)) (not (Widget|IsVisible (Variables|/Script/SherlockProject.TP_ThirdPersonCharacter|Getreportboard (stale EventBeginPlay _astp_third_person_character)))))
    (Widget|SetVisibility (Variables|/Script/SherlockProject.TP_ThirdPersonCharacter|Getreportboard (stale EventBeginPlay _astp_third_person_character)) "Visible")
    ;[1 1 1] 화면 움직임. mouse 보이게
    (Input|SetInputModeUIOnly _returnvalue 0 "DoNotLock" false)
    (Variables|/Script/Engine.PlayerController|SetbShowMouseCursor _returnvalue true)
    (Pawn|Components|CharacterMovement|DisableMovement (Variables|/Script/Engine.Character|GetCharacterMovement (Game|GetPlayerCharacter 0)))))

(fn ConstructionScript)