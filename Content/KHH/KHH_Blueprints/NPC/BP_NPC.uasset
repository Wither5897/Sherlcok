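; BP_NPC is an NPC that shows dialogue lines from an array in a WB_Dialogue widget.
; Talk opens the widget at the current Talkindex and enables the cursor with Game and UI input.
; BeginPlay hides the first BP_NPC found in the level.
; An unconnected chain would advance lines and, after the last, close the widget, hide Mesh and Widget, and restore game input.
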(event EventBeginPlay
  (bind _returnvalue (Actor|GetActorOfClass "BP_NPC_C"))
  (Rendering|SetActorHiddenInGame _returnvalue true))

(event EventTalk
  (bind _returnvalue (Game|GetPlayerController 0))
  (Variables|/Script/Engine.PlayerController|SetbShowMouseCursor _returnvalue true)
  (Input|SetInputModeGameandUI _returnvalue 0 "DoNotLock" true false)
  (bind _returnvalue_2 (UserInterface|CreateWidget "/Game/KHH/KHH_Blueprints/NPC/WB_Dialogue.WB_Dialogue_C" (Game|GetPlayerController 0)))
  (bind _output_get (Variables|Default|SetUI _returnvalue_2))
  (UserInterface|Viewport|AddtoViewport _output_get 0)
  (Rendering|Components|TextRender|SetText (Variables|/Game/KHH/KHH_Blueprints/NPC/WB_Dialogue.WB_Dialogue_C|GetTalkText (Variables|Default|GetUI)) (Utilities|Text|ToText(String) (Utilities|Array|Get(acopy) (Variables|Default|Getdialogue) (Variables|Default|Gettalkindex)))))

(fn ConstructionScript)