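; BP_PhysicSphere is a Blueprint that raises or lowers its Sphere1 component each time the SphereUp event is called.
; IsSphereUp selects one of two timelines, and each update flips the flag so the next call moves the opposite way.
; Each update adds or subtracts a timeline-driven Z offset from the current world location, so movement accumulates per frame rather than interpolating between fixed endpoints.
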(event Custom|Sphere%20Up
  (bind _sphere1 (Variables|Default|GetSphere1))
  (bind _sphere1_2 (Variables|Default|GetSphere1))
  (bind _returnvalue (Transformation|GetWorldLocation _sphere1_2))
  (bind _returnvalue_2 (Transformation|GetWorldLocation _sphere1))
  (if (Variables|Default|GetisSphereUp)
    (bind _newtrack_0 (Timeline|Timeline PlayFromStart)
      (:Update
        (Transformation|SetWorldLocation _sphere1_2 (Math|Vector|MakeVector (.x _returnvalue) (.y _returnvalue) (+ (.z _returnvalue) (Math|Float|Lerp 0.0 1.0 _newtrack_0))) false false)
        (Variables|Default|SetisSphereUp false)))
    (else
      (bind _newtrack_0_2 (Timeline|Timeline_0 PlayFromStart)
        (:Update
          (Transformation|SetWorldLocation _sphere1 (Math|Vector|MakeVector (.x _returnvalue_2) (.y _returnvalue_2) (- (.z _returnvalue_2) (Math|Float|Lerp 0.0 1.0 _newtrack_0_2))) false false)
          (Variables|Default|SetisSphereUp true))))))

(fn ConstructionScript)