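; BP_3dWidget is an actor that shows a login widget in the world through a widget component.
; On BeginPlay it sets game-and-UI input focused on that widget, casts it to BP_TJ_LoginWidget and puts keyboard focus on its host name field.
; The interaction input action presses and releases the WidgetInteraction pointer key, forwarding the pressed key as a click on the 3D UI.
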(event EventBeginPlay
  (bind _widget (Variables|Default|GetWidget))
  (bind _returnvalue (UserInterface|GetUserWidgetObject _widget))
  (Input|SetInputModeGameandUI (Game|GetPlayerController 0) _returnvalue "DoNotLock" true false)
  (bind _asbp_tj_login_widget (Utilities|Casting|CastToBP_TJ_LoginWidget _returnvalue))
  (Widget|SetKeyboardFocus (Variables|/Script/SherlockProject.TJ_LoginWidget|GetEdit_hostName _asbp_tj_login_widget)))

(event Collision|EventActorBeginOverlap
  (params (OtherActor :type Actor%20Object%20Reference)))

(event EventTick
  (params (DeltaSeconds :type Float%20%28single-precision%29)))

(event Input|ActionEvents|InputActioninteraction
  (params (Key :type Key%20Structure :default "None"))
  (bind _widgetinteraction (Variables|Default|GetWidgetInteraction))
  (:Pressed
    (Class|WidgetInteractionComponent|PressPointerKey _widgetinteraction Key))
  (:Released
    (Class|WidgetInteractionComponent|ReleasePointerKey _widgetinteraction Key)))

(fn ConstructionScript)