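; SKBP_Ping is an actor, apparently a waypoint marker, that reacts when the first-person player character touches its sphere.
; BeginPlay caches the player character, and the sphere's begin-overlap event compares the overlapping actor against it.
; On a match it spawns another SKBP_Ping at a hardcoded location, unless it already sits there, then destroys itself.
; The location check ends the chain after that second ping.
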(event OnComponentBeginOverlap(Sphere)
  (params (OverlappedComponent :type Primitive%20Component%20Object%20Reference) (OtherActor :type Actor%20Object%20Reference) (OtherComp :type Primitive%20Component%20Object%20Reference) (OtherBodyIndex :type Integer) (bFromSweep :type Boolean) (SweepResult :type Hit%20Result%20Structure%20%28by%20ref%29))
  (if (== OtherActor (Variables|Default|GetAs%20BP%20First%20Person%20Character))
    (if (Class|KismetMathLibrary|EqualExactlyVectorVector (Transformation|GetActorLocation) "-180.000000,60.000000,280.000000")
      _
      (else
        (Game|SpawnActorfromClass "SKBP_Ping_C" (Math|Transform|MakeTransform "-180.000000,60.000000,280.000000" "0, 0, 0" "1.000000,1.000000,1.000000") "Undefined" "MultiplyWithRoot" 0 0)))
    (Actor|DestroyActor)))

(event EventBeginPlay
  (bind _asbp_first_person_character (Utilities|Casting|CastToBP_FirstPersonCharacter (Game|GetPlayerCharacter 0)))
  (Variables|Default|SetAs%20BP%20First%20Person%20Character _asbp_first_person_character))

(event Collision|EventActorBeginOverlap
  (params (OtherActor :type Actor%20Object%20Reference)))

(event EventTick
  (params (DeltaSeconds :type Float%20%28single-precision%29)))

(fn ConstructionScript)