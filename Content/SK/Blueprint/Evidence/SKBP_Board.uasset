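; SKBP_Board is an evidence board Blueprint that shows an interaction prompt while the first-person player character is within its box trigger.
; On BeginPlay it caches the player character, then creates a WBP_Interaction widget, adds it to the viewport and hides it.
; BoxArea's begin and end overlap events show and hide that widget for the cached character only; no interaction input is handled here.
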(event OnComponentBeginOverlap(BoxArea)
  (params (OverlappedComponent :type Primitive%20Component%20Object%20Reference) (OtherActor :type Actor%20Object%20Reference) (OtherComp :type Primitive%20Component%20Object%20Reference) (OtherBodyIndex :type Integer) (bFromSweep :type Boolean) (SweepResult :type Hit%20Result%20Structure%20%28by%20ref%29))
  (if (== OtherActor (Variables|Default|GetAs%20BP%20First%20Person%20Character))
    (Widget|SetVisibility (Variables|Default|Getinteract%20UI) "Visible")))

(event OnComponentEndOverlap(BoxArea)
  (params (OverlappedComponent :type Primitive%20Component%20Object%20Reference) (OtherActor :type Actor%20Object%20Reference) (OtherComp :type Primitive%20Component%20Object%20Reference) (OtherBodyIndex :type Integer))
  (if (== (Variables|Default|GetAs%20BP%20First%20Person%20Character) OtherActor)
    (Widget|SetVisibility (Variables|Default|Getinteract%20UI) "Hidden")))

(event EventBeginPlay
  (bind _asbp_first_person_character (Utilities|Casting|CastToBP_FirstPersonCharacter (Game|GetPlayerCharacter 0)))
  (Variables|Default|SetAs%20BP%20First%20Person%20Character _asbp_first_person_character)
  (bind _returnvalue (UserInterface|CreateWidget "/Game/KHH/UI/WBP_Interaction.WBP_Interaction_C"))
  (bind _output_get (Variables|Default|Setinteract%20UI _returnvalue))
  (UserInterface|Viewport|AddtoViewport _output_get 0)
  (Widget|SetVisibility _output_get "Hidden"))

(fn ConstructionScript)