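; BP_midnightSun is a sky sphere Blueprint that colors a panning-cloud sky material to match a directional light.
; Its construction script creates the dynamic material, with a RefreshMaterial bool serving as a rerun toggle in the details panel.
; UpdateSunDirection passes light direction and color to the material, then derives sun height from pitch.
; That height samples horizon, zenith and cloud color curves, sets horizon falloff and blends in stars when negative.
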(fn ConstructionScript
  (bind _returnvalue (Rendering|Material|CreateDynamicMaterialInstance (Variables|BP_Skydome|GetSkySphereMesh) 0 "/Engine/EngineSky/M_Sky_Panning_Clouds2.M_Sky_Panning_Clouds2" "None" :!class /Script/Engine.PrimitiveComponent))
  (Variables|Default|SetSky%20material _returnvalue)
  (if (Variables|Default|GetRefresh%20material) ; Updating bool in details panel causes construction script to run again
    _
    (else
      _))
  (Variables|Default|SetRefresh%20material false))

(fn UpdateSunDirection
  (bind _sky_material (Variables|Default|GetSky%20material))
  (bind _sky_material_2 (Variables|Default|GetSky%20material))
  (Rendering|Material|SetVectorParameterValue _sky_material "Light direction" (Math|Conversions|ToLinearColor(Vector) (Math|Rotator|GetRotationXVector (Transformation|GetActorRotation (Variables|Default|GetDirectional%20light%20actor)))) :!class /Script/Engine.MaterialInstanceDynamic)
  (Rendering|Material|SetVectorParameterValue _sky_material "Sun color" (Math|Conversions|ToLinearColor(Color) (Variables|/Script/Engine.LightComponentBase|GetLightColor (Variables|/Script/Engine.Light|GetLightComponent (Variables|Default|GetDirectional%20light%20actor)))) :!class /Script/Engine.MaterialInstanceDynamic)
  (Variables|Default|Setheight_Sun (Math|Float|MapRangeUnclamped (.Pitch (Math|Rotator|BreakRotator (Transformation|GetActorRotation (Variables|Default|GetDirectional%20light%20actor)))) 0.0 -9e+01 0.0 1.0))
  (Rendering|Material|SetVectorParameterValue _sky_material_2 "Horizon color" (Class|CurveLinearColor|GetClampedLinearColorValue (Variables|Default|GetHorizon%20color%20curve) (Variables|Default|Getheight_Sun)) :!class /Script/Engine.MaterialInstanceDynamic)
  (Rendering|Material|SetVectorParameterValue _sky_material_2 "Zenith color" (Class|CurveLinearColor|GetClampedLinearColorValue (Variables|Default|GetZenith%20color%20curve) (Variables|Default|Getheight_Sun)) :!class /Script/Engine.MaterialInstanceDynamic)
  (Rendering|Material|SetVectorParameterValue _sky_material_2 "Cloud color" (Class|CurveLinearColor|GetClampedLinearColorValue (Variables|Default|GetCloud%20color%20curve) (Variables|Default|Getheight_Sun)) :!class /Script/Engine.MaterialInstanceDynamic)
  (Rendering|Material|SetScalarParameterValue _sky_material_2 "Horizon falloff" (Math|Float|Lerp 3.0 8.0 (Math|Float|Absolute(Float) (Variables|Default|Getheight_Sun))) :!class /Script/Engine.MaterialInstanceDynamic)
  (Rendering|Material|SetScalarParameterValue _sky_material_2 "height_Sun" (Math|Float|SelectFloat (Math|Float|Absolute(Float) (Variables|Default|Getheight_Sun)) 0.0 (< (Variables|Default|Getheight_Sun) 0.0)) :!class /Script/Engine.MaterialInstanceDynamic))